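; BP_MarkerActor draws a trail of markers along PathPoints to a target and clears it as the character moves over it.
; On BeginPlay it puts TargetMarker at the last point, fills BasePoints with instances spaced by Subdivide, and adds larger TurningPoints instances at the other path points.
; Each tick, RemoveOvellapedInstances deletes instances from both instanced meshes inside a box around the character's mesh location.
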(event EventBeginPlay
  (bind _pathpoints (Variables|Default|GetPathPoints))
  (bind _output_get (Variables|Default|SetTarget (Utilities|Array|Get(acopy) _pathpoints (Utilities|Array|LastIndex _pathpoints))))
  (Transformation|SetWorldLocation (Variables|Default|GetTargetMarker) _output_get false true)
  (for _array_element (CallFunction|Subdivide _pathpoints 1e+02)
    (Class|InstancedStaticMeshComponent|AddInstanceWorldSpace (Variables|Default|GetBasePoints) (Math|Transform|MakeTransform _array_element "0, 0, 0" "1,1,1")))
  (for _index (range 0 (- (Utilities|Array|Length _pathpoints) 2))
    (Class|InstancedStaticMeshComponent|AddInstanceWorldSpace (Variables|Default|GetTurningPoints) (Math|Transform|MakeTransform (Utilities|Array|Get(acopy) _pathpoints _index) "0, 0, 0" "2.000000,2.000000,2.000000"))))

(event EventTick
  (params (DeltaSeconds :type Float%20%28single-precision%29))
  (bind _character (Variables|Default|GetCharacter))
  (bind _mesh (Variables|/Script/Engine.Character|GetMesh _character))
  (CallFunction|RemoveOvellapedInstances (Variables|Default|GetBasePoints) _mesh)
  (CallFunction|RemoveOvellapedInstances (Variables|Default|GetTurningPoints) _mesh))

(fn ConstructionScript)

(fn Subdivide
  (params (InputPin :type Array%20of%20Vectors) (Distance :type Float%20%28single-precision%29))
  (for _index (range 0 (- (Utilities|Array|Length InputPin) 2))
    (for _index_2 (range 1 (Math|Float|Floor (/ (Math|Vector|Distance(Vector) (Utilities|Array|Get(acopy) InputPin _index) (Utilities|Array|Get(acopy) InputPin (+ _index 1))) Distance)))
      (Utilities|Array|Add (LocalVariables|GetOutput) (+ (Utilities|Array|Get(acopy) InputPin _index) (* (- (Utilities|Array|Get(acopy) InputPin (+ _index 1)) (Utilities|Array|Get(acopy) InputPin _index)) (* _index_2 (/ Distance (Math|Vector|Distance(Vector) (Utilities|Array|Get(acopy) InputPin _index) (Utilities|Array|Get(acopy) InputPin (+ _index 1))))))))))
  (return (LocalVariables|GetOutput)))

(fn RemoveOvellapedInstances
  (params (InstancedStaticMesh :type Hierarchical%20Instanced%20Static%20Mesh%20Component%20Object%20Reference) (ActorComponent :type Scene%20Component%20Object%20Reference))
  (bind _returnvalue (Transformation|GetWorldLocation ActorComponent))
  (Class|HierarchicalInstancedStaticMeshComponent|RemoveInstances InstancedStaticMesh (Class|InstancedStaticMeshComponent|GetInstancesOverlappingBox InstancedStaticMesh (Math|Box|MakeBox (- _returnvalue "50.000000,50.000000,100.000000") (+ _returnvalue "50.000000,50.000000,100.000000")) true)))