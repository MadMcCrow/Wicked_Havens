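; Blueprint function library that starts and ends dialogs between a player-controlled BP_BaseCharacter and an actor with a BP_DialogComponent.
; StartDialogForPlayer accepts the two actors in either order, then passes the component's Dialog to a new WBP_DialogueWidget_Main with UI-only input.
; EndDialogForPlayer removes every widget of that class, not just the player's, and restores Game-and-UI input.
; GetMaxDistanceForDialog returns the component's MinDistance despite its name.
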(fn AddDialogforPlayer
  (params (Player :type Player%20Controller%20Object%20Reference) (Dialog :type BPA%20Dialog%20Asset%20Object%20Reference))
  (bind _returnvalue (UserInterface|CreateWidget "/Game/BLUEPRINT/Dialogs/WBP_DialogueWidget_Main.WBP_DialogueWidget_Main_C" Player Dialog))
  (UserInterface|Viewport|AddtoPlayerScreen _returnvalue)
  (Input|SetInputModeUIOnly Player _returnvalue "LockOnCapture"))

(fn EndDialogforPlayer
  (params (Player :type Player%20Controller%20Object%20Reference))
  (bind _foundwidgets (Widget|GetAllWidgetsOfClass Player "/Game/BLUEPRINT/Dialogs/WBP_DialogueWidget_Main.WBP_DialogueWidget_Main_C" false))
  (for _array_element _foundwidgets
    (Widget|RemovefromParent _array_element)
    (Input|SetInputModeGameandUI Player 0 "DoNotLock" true)))

(fn ActorHasDialog
  (params (Actor :type Actor%20Object%20Reference))
  (Utilities|IsValid Actor
    (:Is%20Valid
      (return (Utilities|IsValid (Actor|GetComponentbyClass Actor "/Game/BLUEPRINT/Dialogs/BP_DialogComponent.BP_DialogComponent_C"))))))

(fn GetDialogfromActor
  (params (Actor :type Actor%20Object%20Reference))
  (Utilities|IsValid Actor
    (:Is%20Valid
      (bind _dialog (Variables|/Game/BLUEPRINT/Dialogs/BP_DialogComponent.BP_DialogComponent_C|GetDialog (Actor|GetComponentbyClass Actor "/Game/BLUEPRINT/Dialogs/BP_DialogComponent.BP_DialogComponent_C"))
        (:then
          (return _dialog true))
        (:else
          (return 0 false))))))

(fn GetMaxDistanceforDialog
  (params (Target :type Actor%20Object%20Reference))
  (bind _returnvalue (Actor|GetComponentbyClass Target "/Game/BLUEPRINT/Dialogs/BP_DialogComponent.BP_DialogComponent_C"))
  (if (Utilities|IsValid _returnvalue)
    (return (Variables|/Game/BLUEPRINT/Dialogs/BP_DialogComponent.BP_DialogComponent_C|GetMinDistance _returnvalue))))

(fn StartDialogforPlayer
  (params (A :type Actor%20Object%20Reference) (B :type Actor%20Object%20Reference))
  (bind (_iscontrolled _playercontroller) (Hidden|ActorIsPlayerControlled A))
  (bind (_iscontrolled_2 _playercontroller_2) (Hidden|ActorIsPlayerControlled B))
  (if (and (Hidden|ActorHasDialog A) _iscontrolled_2)
    (Hidden|AddDialogforPlayer _playercontroller_2 (.Dialog (Hidden|GetDialogfromActor A)))
    (elif (and _iscontrolled (Hidden|ActorHasDialog B))
      (Hidden|AddDialogforPlayer _playercontroller (.Dialog (Hidden|GetDialogfromActor B))))))

(fn ActorIsPlayerControlled
  (params (Object :type Actor%20Object%20Reference))
  (bind (_asbp_base_character _bsuccess) (Utilities|Casting|CastToBP_BaseCharacter Object))
  (bind (_iscontrolledbyplayer _playercontroller) (Default|GetPlayerController _asbp_base_character))
  (Utilities|IsValid Object
    (:Is%20Valid
      (return (and _iscontrolledbyplayer _bsuccess) _playercontroller))))