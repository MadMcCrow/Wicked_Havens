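; Blueprint function library that resolves hostility between clans and decides whether one object should attack another.
; ShouldAttack reads both objects' clans through BPI_ClanInterface, logging an error if either lacks it, and requires a found, specific attitude value.
; GetAlignementToward selects the first clan's data asset and looks up the second in its hostility map, with a fallback when absent.
; Only the Player clan has a data asset assigned.
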(fn GetAlignementToward
  (params (ClanA :type EClan%20Enum :default "NewEnumerator0") (ClanB :type EClan%20Enum :default "NewEnumerator0"))
  (bind _returnvalue (Utilities|Select :Index ClanA :NewEnumerator0 "/Game/DATA/Clans/DA_Clan_Player.DA_Clan_Player" :NewEnumerator5 0 :NewEnumerator1 0 :NewEnumerator2 0 :NewEnumerator3 0 :NewEnumerator4 0))
  (bind _hostilitymap (CallFunction|GetClanHostilityMap _returnvalue))
  (bind (_hostility _found) (CallFunction|GetHostilityfromMap _hostilitymap ClanB))
  (return _hostility _found))

(fn GetClanHostilityMap
  (params (DataAsset :type BP%20Clan%20Data%20Object%20Object%20Reference%20%28by%20ref%29))
  (return (Variables|/Game/BLUEPRINT/Clans/BP_ClanDataObject.BP_ClanDataObject_C|GetHostilityMap DataAsset)))

(fn GetHostilityfromMap
  (params (HostiltyMap :type Map%20of%20EClan%20Enums%20to%20Bytes :default "NewEnumerator0") (Clan :type EClan%20Enum%20%28by%20ref%29 :default "NewEnumerator0"))
  (bind (_value _returnvalue) (Utilities|Map|Find HostiltyMap Clan))
  (if _returnvalue
    (return _value _returnvalue)
    (else
      (return "NewEnumerator2" false))))

(fn ShouldAttack
  (params (A :type Actor%20Object%20Reference) (B :type Actor%20Object%20Reference))
  (if (and (Utilities|DoesObjectImplementInterface A "/Game/BLUEPRINT/Clans/BPI_ClanInterface.BPI_ClanInterface_C") (Utilities|DoesObjectImplementInterface B "/Game/BLUEPRINT/Clans/BPI_ClanInterface.BPI_ClanInterface_C"))
    (bind _clan (Class|BPIClanInterface|GetClan(Message) A))
    (bind _clan_2 (Class|BPIClanInterface|GetClan(Message) B))
    (return (and (Utilities|Enum|Equal(Enum) (.Attitude (CallFunction|GetAlignementToward _clan _clan_2)) "NewEnumerator4") (.Found (CallFunction|GetAlignementToward _clan _clan_2))))
    (else
      (CallFunction|PrintErrorMessage "One of the object does not implement Clans" "BPFL_Clans"))))