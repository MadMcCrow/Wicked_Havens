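; BP_BaseCharacter is the base unit character, which relays orders to its AI controller and exposes its clan.
; OrderToAI casts the controller to BP_AIController and forwards the order with its abort-previous flag, printing an error if the cast fails.
; GetPlayerController casts the character's owner, rather than its controller, to BP_BasePlayerController to report whether a player controls the unit and return that player controller.
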(event Custom|OrderToAI
  (params (Order :type F%20Order%20Info%20Structure) (abortPreviousOrder :type Boolean))
  ;[1 1 1] Passthrougth Orders to AI controller
  (bind _asbp_aicontroller (Utilities|Casting|CastToBP_AIController (Pawn|GetController))
    (:then
      (Default|ReceiveOrder _asbp_aicontroller Order abortPreviousOrder))
    (:CastFailed
      (CallFunction|PrintErrorMessage "Error Invalid Controller Set in :" self))))

(fn ConstructionScript)

(fn GetPlayerController
  (bind _returnvalue (Components|GetOwner))
  (bind (_asbp_base_player_controller _bsuccess) (Utilities|Casting|CastToBP_BasePlayerController _returnvalue))
  (return _bsuccess _asbp_base_player_controller))

(fn GetClan
  (return (Variables|Clan|GetClan)))