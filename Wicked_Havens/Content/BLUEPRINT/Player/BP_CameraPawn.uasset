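; Player camera pawn with axis-driven panning, screen-edge scrolling, spring-arm zoom and a character-follow mode.
; Tick turns normalized mouse position into edge-scroll input for FloatingPawnMovement, scaled by squared zoom distance.
; Zoom input adjusts a clamped ZoomDistance that the arm length interpolates toward.
; Following teleports the pawn to the character each tick and derives zoom from its bounds, until nonzero move or zoom axis input releases it.
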(event Custom|SetFollowCharacter
  (params (CharacterToFollow :type Character%20Object%20Reference))
  (Variables|Default|SetCharacterToFollow CharacterToFollow)
  (Variables|Default|SetbFollowCharacter true)
  (CallFunction|ZoomonActor (Variables|Default|GetCharacterToFollow)))

(event Custom|SetFree
  (Variables|Default|SetbFollowCharacter false))

(event EventTick
  (params (DeltaSeconds :type Float%20%28single-precision%29))
  (bind _edge_movement (CallFunction|BorderMoveDetection 0.05 0.05 true false))
  (CallFunction|MoveCamera _edge_movement (/ (Math|Float|Power (Variables|Zoom|GetZoomDistance) 2.0) 1.5e+06))
  (if (Variables|Default|GetbFollowCharacter)
    (CallFunction|ZoomonActor (Variables|Default|GetCharacterToFollow))))

(event EventBeginPlay
  (Variables|Zoom|SetZoomDistance (Variables|/Script/Engine.SpringArmComponent|GetTargetArmLength (Variables|Default|GetSpringArm))))

(event Input|AxisEvents|InputAxisMoveCameraForward
  (params (AxisValue :type Float%20%28single-precision%29))
  (CallFunction|MoveCamera (Math|Vector|MakeVector AxisValue 0.0 0.0) 4.0)
  (if (!= AxisValue 0.0)
    (CallFunction|SetFree)))

(event Input|AxisEvents|InputAxisMoveCameraRight
  (params (AxisValue :type Float%20%28single-precision%29))
  (CallFunction|MoveCamera (Math|Vector|MakeVector 0.0 AxisValue 0.0) 4.0)
  (if (!= AxisValue 0.0)
    (CallFunction|SetFree)))

(event Input|AxisEvents|InputAxisZoom
  (params (AxisValue :type Float%20%28single-precision%29))
  (CallFunction|Zoom AxisValue 5e+01)
  (if (!= AxisValue 0.0)
    (CallFunction|SetFree)))

(fn ConstructionScript)

(fn BorderMoveDetection
  (params (X_Threshold :type Float%20%28single-precision%29) (Y_Threshold :type Float%20%28single-precision%29) (invertXY :type Boolean) (Outside%20Movement :type Boolean))
  (bind _returnvalue (Class|WidgetLayoutLibrary|GetMousePositiononViewport))
  (Utilities|FlowControl|Sequence
    (:then_0
      (if (or (and (<= (.X (Math|Vector2D|BreakVector2D (/ (* _returnvalue (Class|WidgetLayoutLibrary|GetViewportScale)) (Viewport|GetViewportSize)))) 1.0) (>= (.X (Math|Vector2D|BreakVector2D (/ (* _returnvalue (Class|WidgetLayoutLibrary|GetViewportScale)) (Viewport|GetViewportSize)))) 0.0)) Outside%20Movement)
        (LocalVariables|SetX_Outside (Utilities|BorderMovementMath (Class|KismetMathLibrary|XORBoolean (>= (.x (Class|KismetMathLibrary|ClampAxes2D (/ (* _returnvalue (Class|WidgetLayoutLibrary|GetViewportScale)) (Viewport|GetViewportSize)) 0.0 1.0)) (- 1.0 X_Threshold)) (<= (.x (Class|KismetMathLibrary|ClampAxes2D (/ (* _returnvalue (Class|WidgetLayoutLibrary|GetViewportScale)) (Viewport|GetViewportSize)) 0.0 1.0)) X_Threshold)) (<= (.x (Class|KismetMathLibrary|ClampAxes2D (/ (* _returnvalue (Class|WidgetLayoutLibrary|GetViewportScale)) (Viewport|GetViewportSize)) 0.0 1.0)) X_Threshold) (.x (Class|KismetMathLibrary|ClampAxes2D (/ (* _returnvalue (Class|WidgetLayoutLibrary|GetViewportScale)) (Viewport|GetViewportSize)) 0.0 1.0)) X_Threshold))))
    (:then_1
      (if (or (and (<= (.Y (Math|Vector2D|BreakVector2D (/ (* _returnvalue (Class|WidgetLayoutLibrary|GetViewportScale)) (Viewport|GetViewportSize)))) 1.0) (>= (.Y (Math|Vector2D|BreakVector2D (/ (* _returnvalue (Class|WidgetLayoutLibrary|GetViewportScale)) (Viewport|GetViewportSize)))) 0.0)) Outside%20Movement)
        (LocalVariables|SetY_Outside (* (Utilities|BorderMovementMath (Class|KismetMathLibrary|XORBoolean (>= (.y (Class|KismetMathLibrary|ClampAxes2D (/ (* _returnvalue (Class|WidgetLayoutLibrary|GetViewportScale)) (Viewport|GetViewportSize)) 0.0 1.0)) (- 1.0 Y_Threshold)) (<= (.y (Class|KismetMathLibrary|ClampAxes2D (/ (* _returnvalue (Class|WidgetLayoutLibrary|GetViewportScale)) (Viewport|GetViewportSize)) 0.0 1.0)) Y_Threshold)) (<= (.y (Class|KismetMathLibrary|ClampAxes2D (/ (* _returnvalue (Class|WidgetLayoutLibrary|GetViewportScale)) (Viewport|GetViewportSize)) 0.0 1.0)) Y_Threshold) (.y (Class|KismetMathLibrary|ClampAxes2D (/ (* _returnvalue (Class|WidgetLayoutLibrary|GetViewportScale)) (Viewport|GetViewportSize)) 0.0 1.0)) Y_Threshold) -1.0))))
    (:then_2
      (if invertXY
        (return (Math|Vector|MakeVector (LocalVariables|GetY_Outside) (LocalVariables|GetX_Outside) 0.0))
        (else
          (return (Math|Vector|MakeVector (LocalVariables|GetX_Outside) (LocalVariables|GetY_Outside) 0.0)))))))

(fn MoveCamera
  (params (Value :type Vector) (Scale :type Float%20%28single-precision%29))
  (Class|PawnMovementComponent|AddInputVector (Variables|Default|GetFloatingPawnMovement) (* Value Scale) false))

(fn Zoom
  (params (Delta :type Float%20%28single-precision%29) (Scale :type Float%20%28single-precision%29))
  (Variables|Zoom|SetZoomDistance (Math|Float|Clamp(Float) (+ (* Delta (* Scale -1.0)) (Variables|Zoom|GetZoomDistance)) 2e+02 5e+03))
  (Variables|/Script/Engine.SpringArmComponent|SetTargetArmLength (Variables|Default|GetSpringArm) (Math|Interpolation|FInterpTo (Variables|/Script/Engine.SpringArmComponent|GetTargetArmLength (Variables|Default|GetSpringArm)) (Variables|Zoom|GetZoomDistance) (Utilities|Time|GetWorldDeltaSeconds) 5.0)))

(fn ZoomonActor
  (params (Actor :type Actor%20Object%20Reference))
  (Transformation|SetActorLocation (Transformation|GetActorLocation Actor) false true)
  (Variables|Zoom|SetZoomDistance (* (Math|Vector|VectorLengthXY (.BoxExtent (Collision|GetActorBounds Actor false))) 2.0)))