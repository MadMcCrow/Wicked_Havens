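; Base player controller for click or tap-to-move control of a player character, with P setting the camera pawn to follow it.
; While SetDestination is active, Tick calls GetOrder, which traces under cursor or finger and picks Move, TalkTo or Attack from clan alignment.
; Only Move is acted on, skipping too-close clicks and spawning a marker actor along the synchronously computed nav path.
; Touch toggles movement through a FlipFlop.
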(event Custom|OrderComplete
  (CallFunction|DestroyMarkers))

(event EventTick
  (params (DeltaSeconds :type Float%20%28single-precision%29))
  (Utilities|IsValid (Variables|Default|GetPlayerCharacter)
    (:Is%20Valid
      (if (Variables|Default|GetSetDestination)
        (bind _orderinfo (CallFunction|GetOrder (Variables|Default|GetIsTouch)))
        (switch Utilities|FlowControl|Switch|SwitchonEOrderType (.type _orderinfo)
          (:NewEnumerator1
            (CallFunction|MovetoLocation (.location _orderinfo))))))))

(event EventBeginPlay)

(event Input|ActionEvents|InputActionSetDestination
  (params (Key :type Key%20Structure))
  (:Pressed
    (Variables|Default|SetSetDestination true)
    (Variables|Default|SetIsTouch false :!label _label))
  (:Released
    (Variables|Default|SetSetDestination false)
    (goto _label)))

(event Input|KeyboardEvents|P
  (params (Key :type Key%20Structure))
  (:Pressed
    (Default|SetFollowCharacter (.AsBP%20Camera%20Pawn (Utilities|Casting|CastToBP_CameraPawn (Pawn|GetControlledPawn))) (Variables|Default|GetPlayerCharacter))))

(event Input|TouchEvents|InputTouch
  (params (Location :type Vector) (FingerIndex :type ETouchIndex%20Enum))
  ;[1 1 1] Touch Controls (Tablet and Smartphone)
  (:Pressed
    (Variables|Default|SetIsTouch true :!label _label)
    (if (Utilities|Enum|Equal(Enum) FingerIndex "Touch1")
      (bind _isa (Utilities|FlowControl|FlipFlop)
        (:A
          _)
        (:B
          _))
      (Variables|Default|SetSetDestination _isa)))
  (:Released
    (goto _label)))

(fn ConstructionScript)

(fn MovetoLocation
  (params (Location :type Vector))
  (bind _playercharacter (Variables|Default|GetPlayerCharacter))
  (if (>= (Math|Vector|VectorLength (- (Transformation|GetActorLocation _playercharacter) Location)) (Variables|Default|GetMinClickDistance)) ; Don't move if player clicks too close to pawn
    (Default|Moveto _playercharacter Location)
    (bind _returnvalue (Class|NavigationSystemV1|FindPathtoLocationSynchronously (Transformation|GetActorLocation _playercharacter) Location _playercharacter "/Script/AIModule.NavFilter_AIControllerDefault"))
    (CallFunction|DrawMarkers _returnvalue)))

(fn DrawMarkers
  (params (NavPath :type Navigation%20Path%20Object%20Reference))
  (bind _playercharacter (Variables|Default|GetPlayerCharacter))
  (Utilities|FlowControl|Sequence
    (:then_0
      (CallFunction|DestroyMarkers))
    (:then_1
      (if (and (Utilities|IsValid NavPath) (Utilities|IsValid (Variables|Default|GetPlayerCharacter)))
        (bind _returnvalue (Game|SpawnActorfromClass "/Game/BLUEPRINT/Player/Markers/BP_MarkerActor.BP_MarkerActor_C" (Math|Transform|MakeTransform "0, 0, 0" "0, 0, 0" "1,1,1") "Undefined" (Pawn|GetControlledPawn self) _playercharacter (Variables|/Script/NavigationSystem.NavigationPath|GetPathPoints NavPath) _playercharacter))
        (Variables|Default|SetCurrentMarker _returnvalue)))))

(fn GetOrder
  (params (IsTouch :type Boolean))
  (bind _hitresult (Class|PlayerController|GetHitResultUnderFingerbyChannel "Touch1" "TraceTypeQuery2" true))
  (bind _hitresult_2 (Game|Player|GetHitResultUnderCursorbyChannel "TraceTypeQuery2" true))
  (bind _returnvalue (select IsTouch _hitresult _hitresult_2))
  (bind (_bblockinghit _binitialoverlap _time _distance _location _impactpoint _normal _impactnormal _physmat _hitactor) (Collision|BreakHitResult _returnvalue))
  (Development|PrintString "Hello")
  (if (Utilities|DoesObjectImplementInterface _hitactor "/Game/BLUEPRINT/Units/Common/Clans/BPI_ClanInterface.BPI_ClanInterface_C")
    (bind _clan (Class|BPIClanInterface|GetClan(Message) _hitactor))
    (bind _attitude (CallFunction|GetAlignementToward _clan "NewEnumerator8"))
    (switch Utilities|FlowControl|Switch|SwitchonEHostility _attitude
      (:NewEnumerator1
        _)
      (:NewEnumerator0
        _)
      (:NewEnumerator2
        _)
      (:NewEnumerator3
        (return (Utilities|Struct|MakeFOrderInfo "NewEnumerator0" _location _hitactor)))
      (:NewEnumerator4
        (return (Utilities|Struct|MakeFOrderInfo "NewEnumerator0" _location _hitactor)))
      (:NewEnumerator5
        (return (Utilities|Struct|MakeFOrderInfo "NewEnumerator0" _location _hitactor))))
    (return (Utilities|Struct|MakeFOrderInfo "NewEnumerator3" _location _hitactor))
    (else
      (return (Utilities|Struct|MakeFOrderInfo "NewEnumerator1" _location 0)))))

(fn DestroyMarkers
  (if (Utilities|IsValid (Variables|Default|GetCurrentMarker))
    (Actor|DestroyActor (Variables|Default|GetCurrentMarker))))

(fn GetClan
  (return "NewEnumerator8"))